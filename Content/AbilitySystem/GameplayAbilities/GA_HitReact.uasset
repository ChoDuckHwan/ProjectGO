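; GA_HitReact is a gameplay ability that makes its avatar play a hit reaction when activated.
; It applies the GE_HitReact effect to the owner, then plays the montage the avatar supplies through its CombatInterface.
; When the montage completes, is interrupted or is cancelled, it prints a debug "Hello", removes the effect by its stored handle and ends the ability.
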(event Ability|EventActivateAbility
  (|CallParentFunction)
  (bind _returnvalue (Ability|ApplyGameplayEffectToOwner "/Game/AbilitySystem/GameplayEffect/GE_HitReact.GE_HitReact_C"))
  (Variables|Default|SetActivateHitReactHandle _returnvalue)
  (bind _ascombat_interface (Utilities|Casting|CastToCombatInterface (Ability|GetAvatarActorfromActorInfo)))
  (bind _returnvalue_2 (Class|CombatInterface|GetHitReactMontage _ascombat_interface))
  (|PlayMontageandWaitProxy "None" _returnvalue_2 1.0 "None" true 1.0 0.0 false
    (:OnCompleted
      _)
    (:OnInterrupted
      _)
    (:OnCancelled
      _))
  (Development|PrintString "Hello")
  (Ability|RemoveGameplayEffectFromOwnerWithHandle (Variables|Default|GetActivateHitReactHandle))
  (Ability|EndAbility))

(event Ability|EventOnEndAbility
  (params (bWasCancelled :type Boolean)))