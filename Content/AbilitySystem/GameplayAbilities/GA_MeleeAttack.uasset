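; Melee attack gameplay ability that plays a random attack montage and damages nearby hostile live players.
; Montages, combat target and socket location come from avatar interface messages, and facing updates toward the target as the montage starts.
; The montage's gameplay tag event triggers a sphere query at that socket, with debug drawing, and non-friends take damage.
; The ability ends shortly after the hit, or when the montage completes, is interrupted or cancelled.
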(event Ability|EventActivateAbility
  (bind _returnvalue (Ability|GetAvatarActorfromActorInfo))
  (bind _returnvalue_2 (Ability|GetAvatarActorfromActorInfo))
  (|CallParentFunction)
  (bind _returnvalue_3 (Class|CombatInterface|GetAttackMontages(Message) (Ability|GetAvatarActorfromActorInfo)))
  (Variables|Default|SetSelectedMontage (.OutItem (Utilities|Array|Random _returnvalue_3)))
  (|PlayMontageandWaitProxy "None" (.montage (Variables|Default|GetSelectedMontage)) 1.0 "None" true 1.0 0.0 false
    (:then
      (bind _returnvalue_4 (Class|MonsterInterface|GetCombatTarget(Message) _returnvalue))
      (Class|CombatInterface|UpdateFacingTarget(Message) _returnvalue (Transformation|GetActorLocation _returnvalue_4))
      (Ability|Tasks|WaitGameplayEvent (.montagetag (Variables|Default|GetSelectedMontage)) 0
        (:EventReceived
          (bind _returnvalue_5 (Class|CombatInterface|GetCombatSocketLocation(Message) _returnvalue_2 (.montagetag (Variables|Default|GetSelectedMontage))))
          (Rendering|Debug|DrawDebugSphere _returnvalue_5 5e+01 12 "(R=1.000000,G=1.000000,B=1.000000,A=1.000000)" 1.0)
          (bind _outoverlappingactors (Class|GOAbilityBFL|GetLivePlayerswithinRadius _returnvalue_2 (Utilities|Array|MakeArray _returnvalue_2) 5e+01 _returnvalue_5))
          (for _array_element _outoverlappingactors
            (if (Class|GOAbilityBFL|IsNotFriend (Ability|GetAvatarActorfromActorInfo) _array_element)
              (Class|GODamageGameplayAbility|CauseDamage _array_element)))
          (Utilities|FlowControl|Delay 0.2)
          (Ability|EndAbility))))
    (:OnCompleted
      (Ability|EndAbility :!label _label))
    (:OnInterrupted
      (goto _label))
    (:OnCancelled
      (goto _label))))

(event Ability|EventOnEndAbility
  (params (bWasCancelled :type Boolean)))