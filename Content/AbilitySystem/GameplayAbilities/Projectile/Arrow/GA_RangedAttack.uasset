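; Gameplay ability for a ranged attack that fires a projectile at the avatar's combat target.
; On activation it turns the avatar to face the target and plays a montage picked at random from its attack montages.
; A gameplay event wait on a montage tag from that random selection triggers the projectile spawn toward the target's location, then ends the ability.
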(event Ability|EventActivateAbility
  (bind _returnvalue (Class|MonsterInterface|GetCombatTarget(Message) (Ability|GetAvatarActorfromActorInfo)))
  (Class|CombatInterface|UpdateFacingTarget(Message) (Ability|GetAvatarActorfromActorInfo) (Transformation|GetActorLocation _returnvalue))
  (bind _returnvalue_2 (Class|CombatInterface|GetAttackMontages(Message) (Ability|GetAvatarActorfromActorInfo)))
  (|PlayMontageandWaitProxy "None" (.montage (.OutItem (Utilities|Array|Random _returnvalue_2))) 1.0 "None" true 1.0 0.0 false
    (:then
      (Ability|Tasks|WaitGameplayEvent (.montagetag (.OutItem (Utilities|Array|Random _returnvalue_2))) 0
        (:EventReceived
          (Class|GOProjectileSpell|SpawnProjectile (Transformation|GetActorLocation _returnvalue))
          (Ability|EndAbility))))))

(event Ability|EventOnEndAbility
  (params (bWasCancelled :type Boolean)))