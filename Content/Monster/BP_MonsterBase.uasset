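; BP_MonsterBase is a monster base Blueprint that makes the monster a mouse-clickable attack target.
; Clicking it sends the touched actor to player 0's controlled pawn through an ITargetAttack message, while cursor hover begin and end are reported to that player's controller.
; UpdateFacingTarget sets the "FacingTarget" Motion Warping target from a given location and a fixed rotation.
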(event Collision|EventActorBeginOverlap
  (params (OtherActor :type Actor%20Object%20Reference)))

(event EventCharacteronClicked
  (params (TouchedActor :type Actor%20Object%20Reference) (ButtonPressed :type Key%20Structure :default "None"))
  (Class|BPICharacter|ITargetAttack(Message) (Pawn|GetControlledPawn (Game|GetPlayerController 0)) TouchedActor))

(event EventCharacterCursorBeginOvered
  (params (TouchedActor :type Actor%20Object%20Reference))
  (Class|BPIPlayerController|MouseHoverCharacter(Message) (Game|GetPlayerController 0) true))

(event EventCharacterCursorEndOvered
  (params (TouchedActor :type Actor%20Object%20Reference))
  (Class|BPIPlayerController|MouseHoverEndCharacter(Message) (Game|GetPlayerController 0)))

(event EventUpdateFacingTarget
  (params (Target :type Vector%20%28by%20ref%29 :default "0, 0, 0"))
  (Class|MotionWarpingComponent|AddorUpdateWarpTargetfromLocationandRotation (Variables|Default|GetMotionWarping) "FacingTarget" Target "0.000000,270.000000,0.000000"))

(fn ConstructionScript)