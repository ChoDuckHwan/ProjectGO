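; Ranged skeleton enemy Blueprint that carries a bow as its weapon.
; The Construction Script passes the bow mesh to SetWeaponMesh, and this file adds no active runtime logic of its own.
; Unconnected leftover nodes cover bow animation playback, a weapon-tip socket debug print, and leader-pose setup with per-part visibility toggles for modular armor, rags and gear.
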(event EventTick
  (params (DeltaSeconds :type Float%20%28single-precision%29)))

(fn ConstructionScript
  (Class|ProjectGOCharacter|SetWeaponMesh (Variables|Default|GetSK_Bow)))