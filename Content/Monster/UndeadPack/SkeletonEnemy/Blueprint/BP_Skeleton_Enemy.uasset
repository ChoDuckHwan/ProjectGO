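; Skeleton enemy Blueprint with modular armor, clothing and weapon parts plus a particle effect, each with its own visibility variable.
; Its construction graph holds a leader-pose link to the main Mesh, then a Sequence applying those visibility variables to the parts.
; Arrows and bow propagate visibility to their children.
; The Construction Script entry is unconnected to this chain, so none of this setup runs.
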(fn ConstructionScript)