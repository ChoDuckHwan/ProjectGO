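; In-game HUD Blueprint that sets up a custom widget mouse cursor and the player's input mode.
; On BeginPlay it creates the cursor widget, assigns it as the player controller's default cursor, and sets Game-and-UI input with the mouse always locked and visible during capture.
; OnChangeMouseCursorType stores the requested cursor type and forwards it to the WBP_MouseCursor widget to switch the cursor.
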(event EventBeginPlay
  (|CallParentFunction)
  (CallFunction|InitializeMouseCursor)
  (CallFunction|InitializeinGameHud))

(event Collision|EventActorBeginOverlap
  (params (OtherActor :type Actor%20Object%20Reference)))

(event EventTick
  (params (DeltaSeconds :type Float%20%28single-precision%29)))

(event EventOnChangeMouseCursorType
  (params (MouseCursorType :type GO%20Mouse%20Cursor%20Widget%20Class%20Reference))
  (Variables|Default|SetCurrentMouseCursorType MouseCursorType)
  (Utilities|IsValid (Variables|Default|GetMouseCursorIconObjs)
    (:Is%20Valid
      (bind _aswbp_mouse_cursor (Utilities|Casting|CastToWBP_MouseCursor (Variables|Default|GetMouseCursorIconObjs)))
      (Default|ChangeMouseCursorType _aswbp_mouse_cursor (Variables|Default|GetCurrentMouseCursorType)))))

(fn ConstructionScript)

(fn InitializeMouseCursor
  (bind _returnvalue (UserInterface|CreateWidget (Variables|Default|GetCurrentMouseCursorType) (Game|GetPlayerController 0)))
  (bind _output_get (Variables|Default|SetMouseCursorIconObjs _returnvalue))
  (Class|PlayerController|SetMouseCursorWidget (Game|GetPlayerController 0) "Default" _output_get))

(fn InitializeinGameHud
  (Input|SetInputModeGameandUI (Game|GetPlayerController 0) 0 "LockAlways" false true))