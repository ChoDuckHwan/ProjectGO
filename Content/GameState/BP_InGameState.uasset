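; In-game GameState Blueprint that holds a reference to the level's PathFinderVolume and exposes it through an interface getter.
; On BeginPlay, only the non-authority (Remote) branch finds the first PathFinderVolume, stores it and sets itself as that volume's owner, before calling the parent BeginPlay.
; The IPathfindInitialize event and Tick are empty.
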(event EventBeginPlay
  (Utilities|FlowControl|Sequence
    (:then_0
      (Networking|SwitchHasAuthority
        (:Remote
          (bind _outactors (Actor|GetAllActorsOfClass "/Script/ProjectGO.PathFinderVolume"))
          (Class|GOGameState|SetPathFinderVolume (Utilities|Array|Get(acopy) _outactors))
          (Actor|SetOwner (Utilities|Array|Get(acopy) _outactors) self))))
    (:then_1
      (|CallParentFunction))))

(event EventTick
  (params (DeltaSeconds :type Float%20%28single-precision%29)))

(event EventIPathfindInitialize)

(fn ConstructionScript
  (|CallParentFunction))

(fn IGetPathFinderVolume
  (return (Class|GOGameState|GetPathFinderVolume)))