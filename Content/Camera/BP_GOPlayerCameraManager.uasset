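; Player camera manager that provides mouse edge scrolling and smooth FOV zoom, centering the cursor on BeginPlay.
; CameraMoveMouseX/Y compare cursor position to viewport edges, with a wider band at the top, and call AddCameraLocation at a frame-rate-scaled speed, mapping screen X/Y to world Y/X.
; SetCameraFOVSmooth uses a timeline to lerp FOV by the wheel value within min/max limits.
; Tick is unused, so these events rely on external callers.
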(event EventBeginPlay
  (bind _returnvalue (Viewport|GetViewportSize))
  (|CallParentFunction)
  (Class|PlayerController|SetMouseLocation (Game|GetPlayerController 0) (Math|Float|Truncate (* (.x _returnvalue) 0.5)) (Math|Float|Truncate (* (.y _returnvalue) 0.5))))

(event Collision|EventActorBeginOverlap
  (params (OtherActor :type Actor%20Object%20Reference)))

(event EventTick
  (params (DeltaSeconds :type Float%20%28single-precision%29)))

(event EventSetCameraFOVSmooth
  (params (WheelValue :type Float%20%28single-precision%29%20%28by%20ref%29))
  (Variables|Default|SetBeforeFOV (Camera|GetFOVAngle))
  (if (!= WheelValue 0.0)
    (bind _alpha (Timeline|TL_CameraFOV PlayFromStart)
      (:Update
        (Class|GOPlayerCameraManager|SetFOV (Math|Float|Clamp(Float) (Math|Float|Lerp (Variables|Default|GetBeforeFOV) (+ (Variables|Default|GetBeforeFOV) (* WheelValue -1.0 5e+01)) _alpha) (Variables|Default|GetFOVMin) (Variables|Default|GetFOVMax)))))))

(event EventCameraMoveMouseX
  (bind _returnvalue (Utilities|Time|GetWorldDeltaSeconds))
  (bind _returnvalue_2 (Viewport|GetViewportSize))
  (bind _returnvalue_3 (Game|GetPlayerController 0))
  (bind _cameramovescale (Variables|Default|GetCameraMoveScale))
  (bind _locationx (Game|Player|GetMousePosition _returnvalue_3))
  (bind _returnvalue_4 (* _cameramovescale _returnvalue))
  (bind _returnvalue_5 (* "(X=-1.000000,Y=0.000000)" (Math|Vector2D|MakeVector2D _returnvalue_4 _returnvalue_4)))
  (bind _returnvalue_6 (* "(X=1.000000,Y=0.000000)" (Math|Vector2D|MakeVector2D _returnvalue_4 _returnvalue_4)))
  (bind _returnvalue_7 (/ _locationx (.x _returnvalue_2)))
  (Utilities|FlowControl|Sequence
    (:then_0
      (if (> _returnvalue_7 0.995)
        (Class|GOPlayerCameraManager|AddCameraLocation (Math|Vector|MakeVector (.y _returnvalue_6) (.x _returnvalue_6) 0.0))))
    (:then_1
      (if (< _returnvalue_7 0.005)
        (Class|GOPlayerCameraManager|AddCameraLocation (Math|Vector|MakeVector (.y _returnvalue_5) (.x _returnvalue_5) 0.0))))))

(event EventCameraMoveMouseY
  (bind _returnvalue (Game|GetPlayerController 0))
  (bind _returnvalue_2 (Viewport|GetViewportSize))
  (bind _returnvalue_3 (Utilities|Time|GetWorldDeltaSeconds))
  (bind _cameramovescale (Variables|Default|GetCameraMoveScale))
  (bind _locationy (Game|Player|GetMousePosition _returnvalue))
  (bind _returnvalue_4 (* _cameramovescale _returnvalue_3))
  (bind _returnvalue_5 (* "(X=0.000000,Y=1.000000)" (Math|Vector2D|MakeVector2D _returnvalue_4 _returnvalue_4)))
  (bind _returnvalue_6 (* "(X=0.000000,Y=-1.000000)" (Math|Vector2D|MakeVector2D _returnvalue_4 _returnvalue_4)))
  (bind _returnvalue_7 (/ _locationy (.y _returnvalue_2)))
  (Utilities|FlowControl|Sequence
    (:then_0
      (if (< _returnvalue_7 0.05)
        (Class|GOPlayerCameraManager|AddCameraLocation (Math|Vector|MakeVector (.y _returnvalue_5) (.x _returnvalue_5) 0.0))))
    (:then_1
      (if (> _returnvalue_7 0.995)
        (Class|GOPlayerCameraManager|AddCameraLocation (Math|Vector|MakeVector (.y _returnvalue_6) (.x _returnvalue_6) 0.0))))))

(fn ConstructionScript)