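; BP_PathFindGameMode is a game mode that gives each joining player a BP_PathFindCharacter to control.
; HandleStartingNewPlayer calls the parent handler, spawns the character at the location returned by FindPlayerStart, then has the new player controller possess it.
; The spawn takes only the start point's location, not its rotation.
; BeginPlay, Tick and the construction script add no logic of their own.
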(event EventBeginPlay
  (|CallParentFunction) ; 지금 이 노드는 비활성 상태입니다. \n핀을 끌어서 다른 노드를 연결하면 활성화됩니다.
)

(event EventTick
  (params (DeltaSeconds :type Float%20%28single-precision%29))
  (|CallParentFunction DeltaSeconds) ; 지금 이 노드는 비활성 상태입니다. \n핀을 끌어서 다른 노드를 연결하면 활성화됩니다.
)

(event EventHandleStartingNewPlayer
  (params (NewPlayer :type Player%20Controller%20Object%20Reference))
  (|CallParentFunction NewPlayer)
  (bind _returnvalue (Game|SpawnActorfromClass "/Game/Characters/BP_PathFindCharacter.BP_PathFindCharacter_C" (Math|Transform|MakeTransform (Transformation|GetActorLocation (Class|GameModeBase|FindPlayerStart)) "0, 0, 0" "1.000000,1.000000,1.000000") "Undefined" "MultiplyWithRoot" 0 0))
  (Pawn|Possess NewPlayer _returnvalue))

(fn ConstructionScript
  (|CallParentFunction))