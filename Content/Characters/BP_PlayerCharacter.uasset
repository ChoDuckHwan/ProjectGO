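; Player character Blueprint that handles navigation movement and targeted attacks through the Gameplay Ability System.
; NavigationMove converts a synchronous navmesh path into 2D points for the PathFinder component.
; An attack command stores the target, then either stops or moves toward it using GameState grid indices; server-side AttackSphere checks trigger the tagged attack ability when in range.
; Motion Warping updates a facing target for root-motion animations.
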(event OnComponentBeginOverlap(AttackSphere)
  (params (OverlappedComponent :type Primitive%20Component%20Object%20Reference) (OtherActor :type Actor%20Object%20Reference) (OtherComp :type Primitive%20Component%20Object%20Reference) (OtherBodyIndex :type Integer) (bFromSweep :type Boolean) (SweepResult :type Hit%20Result%20Structure%20%28by%20ref%29))
  (Networking|SwitchHasAuthority
    (:Authority
      (if (and (== OtherActor (Variables|Default|GetAttackTarget)) (Variables|Default|GetAttackMove))
        (CallFunction|NormalAttack)))))

(event Custom|NormalAttack
  (Abilities|TryActivateAbilitiesbyTag (Ability|GetAbilitySystemComponent 0) (GameplayTags|MakeLiteralGameplayTagContainer "(GameplayTags=((TagName=\"Ability.Character.Attack\")))") true))

(event Custom|TargetAttack_Server
  (params (TargetActor :type Actor%20Object%20Reference))
  (bind _output_get (Variables|Default|SetAttackTarget TargetActor))
  (if (Collision|IsOverlappingActor (Variables|Default|GetAttackSphere) _output_get :!class /Script/Engine.PrimitiveComponent)
    (CallFunction|NormalAttack)))

(event EventUpdateFacingTarget
  (params (Target :type Vector%20%28by%20ref%29 :default "0, 0, 0"))
  ;[1 1 1] Animation must rootmotion true
  (Class|MotionWarpingComponent|AddorUpdateWarpTargetfromLocation (Variables|Default|GetMotionWarping) "FacingTarget" Target))

(event Collision|EventActorBeginOverlap
  (params (OtherActor :type Actor%20Object%20Reference)))

(event EventITargetAttack
  (params (TargetActor :type Actor%20Object%20Reference))
  (bind _returnvalue (Transformation|GetActorLocation))
  (CallFunction|TargetAttackServer TargetActor)
  (if (Collision|IsOverlappingActor (Variables|Default|GetAttackSphere) TargetActor :!class /Script/Engine.PrimitiveComponent)
    (Class|PathFinderComponent|Stop (Variables|Default|GetPathFinder))
    (else
      (Variables|Default|SetAttackTarget TargetActor)
      (bind _pathfindervolume (Class|IGameState|IGetPathFinderVolume(Message) (Game|GetGameState)))
      (CallFunction|MoveCharacter (Class|PathFinderVolume|GetGridArrayIndexbyLocation _pathfindervolume (Math|Vector2D|MakeVector2D (.x _returnvalue) (.y _returnvalue))) (Class|PathFinderVolume|GetGridArrayIndexbyLocation _pathfindervolume (Math|Vector2D|MakeVector2D (.x (Transformation|GetActorLocation (Variables|Default|GetAttackTarget))) (.y (Transformation|GetActorLocation (Variables|Default|GetAttackTarget))))) (Math|Vector2D|MakeVector2D (.x (Transformation|GetActorLocation (Variables|Default|GetAttackTarget))) (.y (Transformation|GetActorLocation (Variables|Default|GetAttackTarget)))) true))))

(event EventMoveCharacter
  (params (StartIndex :type Integer) (TargetIndex :type Integer) (FinalLocation :type Vector%202D%20Structure) (AttackMove :type Boolean))
  (CallFunction|NavigationMove FinalLocation))

(event EventTick
  (params (DeltaSeconds :type Float%20%28single-precision%29))
  (|CallParentFunction DeltaSeconds))

(fn ConstructionScript
  (|CallParentFunction))

(fn NavigationMove
  (params (InVec :type Vector%202D%20Structure))
  (bind (_x _y) (Math|Vector2D|BreakVector2D InVec))
  (bind _returnvalue (Class|NavigationSystemV1|FindPathtoLocationSynchronously (Class|NavigationSystemV1|GetNavigationSystem) (Transformation|GetActorLocation) (Math|Vector|MakeVector _x _y 0.0) 0 0))
  (Utilities|IsValid _returnvalue
    (:Is%20Valid
      (for _array_element (Variables|/Script/NavigationSystem.NavigationPath|GetPathPoints _returnvalue)
        (Utilities|Array|Add (LocalVariables|Get2D_PathPoints) (Math|Vector2D|MakeVector2D (.x _array_element) (.y _array_element))))
      (Class|PathFinderComponent|Navigate (Variables|Default|GetPathFinder) (LocalVariables|Get2D_PathPoints)))
    (:Is%20Not%20Valid
      (Development|PrintString "Navigation Is In Valid"))))