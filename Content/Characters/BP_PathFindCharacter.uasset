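; Networked character that moves along grid paths and performs normal attacks on targets.
; MoveCharacter navigates via its PathFinder over the GameState's grid volume, then relays the destination through the server so non-controlling clients recompute the path themselves.
; Target attacks stop movement when in range, otherwise path toward the target.
; The server activates the Gameplay Ability attack by tag when the target is inside or enters the AttackSphere during an attack move.
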(event OnComponentBeginOverlap(AttackSphere)
  (params (OverlappedComponent :type Primitive%20Component%20Object%20Reference) (OtherActor :type Actor%20Object%20Reference) (OtherComp :type Primitive%20Component%20Object%20Reference) (OtherBodyIndex :type Integer) (bFromSweep :type Boolean) (SweepResult :type Hit%20Result%20Structure%20%28by%20ref%29))
  (Networking|SwitchHasAuthority
    (:Authority
      (if (and (== OtherActor (Variables|Default|GetAttackTarget)) (Variables|Default|GetAttackMove))
        (CallFunction|NormalAttack)))))

(event Custom|NormalAttack
  (Abilities|TryActivateAbilitiesbyTag (Ability|GetAbilitySystemComponent 0) (GameplayTags|MakeLiteralGameplayTagContainer "(GameplayTags=((TagName=\"Ability.Character.Attack\")))") true))

(event Custom|OtherCharacterMove_Server
  (params (Location :type Vector%202D%20Structure) (AttackMove :type Boolean))
  (CallFunction|OtherCharacterMoveMulticast Location)
  (Variables|Default|SetAttackMove AttackMove))

(event Custom|OtherCharacterMove_Multicast
  (params (Location :type Vector%202D%20Structure))
  (bind _returnvalue (Transformation|GetActorLocation))
  (Networking|SwitchHasAuthority
    (:Remote
      (if (!= (Pawn|GetControlledPawn (Game|GetPlayerController 0)) self)
        (bind _pathfindervolume (Class|IGameState|IGetPathFinderVolume(Message) (Game|GetGameState)))
        (bind _returnvalue_2 (Class|PathFinderComponent|FindPath (Variables|Default|GetPathFinder) (Class|PathFinderVolume|GetGrids _pathfindervolume) (Class|PathFinderVolume|GetGridArrayIndexbyLocation _pathfindervolume (Math|Vector2D|MakeVector2D (.x _returnvalue) (.y _returnvalue))) (Class|PathFinderVolume|GetGridArrayIndexbyLocation _pathfindervolume (Math|Vector2D|MakeVector2D (.x Location) (.y Location))) (Math|Float|Truncate (/ (.y (Variables|/Script/ProjectGO.PathFinderVolume|GetMapSize _pathfindervolume)) (.y (Variables|/Script/ProjectGO.PathFinderVolume|GetGridSize _pathfindervolume)))) (Math|Vector2D|MakeVector2D (.x Location) (.y Location))))
        (Class|PathFinderComponent|Navigate (Variables|Default|GetPathFinder) _returnvalue_2)))))

(event Custom|TargetAttack_Server
  (params (TargetActor :type Actor%20Object%20Reference))
  (bind _output_get (Variables|Default|SetAttackTarget TargetActor))
  (if (Collision|IsOverlappingActor (Variables|Default|GetAttackSphere) _output_get :!class /Script/Engine.PrimitiveComponent)
    (CallFunction|NormalAttack)))

(event Collision|EventActorBeginOverlap
  (params (OtherActor :type Actor%20Object%20Reference)))

(event EventITargetAttack
  (params (TargetActor :type Actor%20Object%20Reference))
  (bind _returnvalue (Transformation|GetActorLocation))
  (CallFunction|TargetAttackServer TargetActor)
  (if (Collision|IsOverlappingActor (Variables|Default|GetAttackSphere) TargetActor :!class /Script/Engine.PrimitiveComponent)
    (Class|PathFinderComponent|Stop (Variables|Default|GetPathFinder))
    (else
      (Variables|Default|SetAttackTarget TargetActor)
      (bind _pathfindervolume (Class|IGameState|IGetPathFinderVolume(Message) (Game|GetGameState)))
      (CallFunction|MoveCharacter (Class|PathFinderVolume|GetGridArrayIndexbyLocation _pathfindervolume (Math|Vector2D|MakeVector2D (.x _returnvalue) (.y _returnvalue))) (Class|PathFinderVolume|GetGridArrayIndexbyLocation _pathfindervolume (Math|Vector2D|MakeVector2D (.x (Transformation|GetActorLocation (Variables|Default|GetAttackTarget))) (.y (Transformation|GetActorLocation (Variables|Default|GetAttackTarget))))) (Math|Vector2D|MakeVector2D (.x (Transformation|GetActorLocation (Variables|Default|GetAttackTarget))) (.y (Transformation|GetActorLocation (Variables|Default|GetAttackTarget)))) true))))

(event EventMoveCharacter
  (params (StartIndex :type Integer) (TargetIndex :type Integer) (FinalLocation :type Vector%202D%20Structure) (AttackMove :type Boolean))
  (bind _pathfindervolume (Class|IGameState|IGetPathFinderVolume(Message) (Game|GetGameState)))
  (Utilities|FlowControl|Sequence
    (:then_0
      (bind _returnvalue (Class|PathFinderComponent|FindPath (Variables|Default|GetPathFinder) (Class|PathFinderVolume|GetGrids _pathfindervolume) StartIndex TargetIndex (Math|Float|Truncate (/ (.y (Variables|/Script/ProjectGO.PathFinderVolume|GetMapSize _pathfindervolume)) (.y (Variables|/Script/ProjectGO.PathFinderVolume|GetGridSize _pathfindervolume)))) FinalLocation))
      (Class|PathFinderComponent|Navigate (Variables|Default|GetPathFinder) _returnvalue))
    (:then_1
      (CallFunction|OtherCharacterMoveServer FinalLocation AttackMove))))

(event EventTick
  (params (DeltaSeconds :type Float%20%28single-precision%29))
  (|CallParentFunction DeltaSeconds))

(fn ConstructionScript
  (|CallParentFunction))