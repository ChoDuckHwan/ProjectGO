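; BP_CharacterBase is a base character Blueprint that makes characters clickable attack targets and hover-aware.
; Clicking it sends an interface target-attack message to the first player's controlled pawn, passing the clicked actor.
; Cursor enter and leave events notify the player controller through hover interface messages.
; The construction script sizes the AttackSphere component from the AttackRange variable.
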(event EventBeginPlay
  (|CallParentFunction))

(event EventCharacteronClicked
  (params (TouchedActor :type Actor%20Object%20Reference) (ButtonPressed :type Key%20Structure :default "None"))
  (Class|BPICharacter|ITargetAttack(Message) (Pawn|GetControlledPawn (Game|GetPlayerController 0)) TouchedActor))

(event EventCharacterCursorBeginOvered
  (params (TouchedActor :type Actor%20Object%20Reference))
  (Class|BPIPlayerController|MouseHoverCharacter(Message) (Game|GetPlayerController 0) true))

(event EventCharacterCursorEndOvered
  (params (TouchedActor :type Actor%20Object%20Reference))
  (Class|BPIPlayerController|MouseHoverEndCharacter(Message) (Game|GetPlayerController 0)))

(fn ConstructionScript
  (|CallParentFunction)
  (Components|Sphere|SetSphereRadius (Variables|Default|GetAttackSphere) (Variables|Default|GetAttackRange) true))