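; Player controller for click-to-move and attack-move of the controlled pawn, with camera panning, zoom and an attribute menu.
; Clicks trace under the cursor, convert pawn and hit locations to grid indices through the GameState's pathfinder volume, and send a move message to the pawn.
; The attack icon input arms an aim cursor; the attack click then attack-moves and spawns a tinted Niagara cursor effect.
; Keyboard, mouse and wheel input drive GOPlayerCameraManager.
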(event Input|EnhancedActionEvents|EnhancedInputActionIA_AttackIcon
  (params (ActionValue :type Boolean) (ElapsedSeconds :type Float%20%28double-precision%29) (TriggeredSeconds :type Float%20%28double-precision%29) (InputAction :type Input%20Action%20Object%20Reference :default "/Game/Input/Actions/IA_AttackIcon.IA_AttackIcon"))
  (:Started
    (bind _asgohudbase (Utilities|Casting|CastToGOHUDBase (HUD|GetHUD)))
    (Class|GOHUDBase|OnChangeMouseCursorTypeImplementation _asgohudbase "/Script/ProjectGO.GOAimCursorType")
    (Variables|Default|SetbCursorAttack true)))

(event Input|EnhancedActionEvents|EnhancedInputActionIA_MoveScreenKeyboard
  (params (ActionValue :type Vector%202D%20Structure) (ElapsedSeconds :type Float%20%28double-precision%29) (TriggeredSeconds :type Float%20%28double-precision%29) (InputAction :type Input%20Action%20Object%20Reference :default "/Game/Input/Actions/IA_MoveScreenKeyboard.IA_MoveScreenKeyboard"))
  (bind _asgoplayer_camera_manager (Utilities|Casting|CastToGOPlayerCameraManager (Game|GetPlayerCameraManager 0)))
  (Class|GOPlayerCameraManager|AddCameraLocation _asgoplayer_camera_manager (Math|Vector|MakeVector (.y (* ActionValue (Math|Vector2D|MakeVector2D (* (Variables|/Script/ProjectGO.GOPlayerCameraManager|GetCameraMoveScale _asgoplayer_camera_manager) (Utilities|Time|GetWorldDeltaSeconds)) (* (Variables|/Script/ProjectGO.GOPlayerCameraManager|GetCameraMoveScale _asgoplayer_camera_manager) (Utilities|Time|GetWorldDeltaSeconds))))) (.x (* ActionValue (Math|Vector2D|MakeVector2D (* (Variables|/Script/ProjectGO.GOPlayerCameraManager|GetCameraMoveScale _asgoplayer_camera_manager) (Utilities|Time|GetWorldDeltaSeconds)) (* (Variables|/Script/ProjectGO.GOPlayerCameraManager|GetCameraMoveScale _asgoplayer_camera_manager) (Utilities|Time|GetWorldDeltaSeconds))))) 0.0)))

(event Input|EnhancedActionEvents|EnhancedInputActionIA_SetDestination_Click
  (params (ActionValue :type Boolean) (ElapsedSeconds :type Float%20%28double-precision%29) (TriggeredSeconds :type Float%20%28double-precision%29) (InputAction :type Input%20Action%20Object%20Reference :default "/Game/Input/Actions/IA_SetDestination_Click.IA_SetDestination_Click"))
  (bind _returnvalue (Pawn|GetControlledPawn))
  (bind (_hitresult _returnvalue_2) (Game|Player|GetHitResultUnderCursorbyChannel "TraceTypeQuery1" true))
  (bind (_x _y) (Math|Vector|BreakVector (.location _hitresult)))
  (bind _returnvalue_3 (Transformation|GetActorLocation _returnvalue))
  (:Started
    (bind _pathfindervolume (Class|IGameState|IGetPathFinderVolume(Message) (Game|GetGameState)))
    (if _returnvalue_2
      (Class|BPICharacter|MoveCharacter(Message) (Pawn|GetControlledPawn) (Class|PathFinderVolume|GetGridArrayIndexbyLocation _pathfindervolume (Math|Vector2D|MakeVector2D (.x _returnvalue_3) (.y _returnvalue_3))) (Class|PathFinderVolume|GetGridArrayIndexbyLocation _pathfindervolume (Math|Vector2D|MakeVector2D _x _y)) (Math|Vector2D|MakeVector2D _x _y) false)
      (Variables|Default|SetbCursorAttack false))))

(event Input|EnhancedActionEvents|EnhancedInputActionIA_AttackClick
  (params (ActionValue :type Boolean) (ElapsedSeconds :type Float%20%28double-precision%29) (TriggeredSeconds :type Float%20%28double-precision%29) (InputAction :type Input%20Action%20Object%20Reference :default "/Game/Input/Actions/IA_AttackClick.IA_AttackClick"))
  (bind (_hitresult _returnvalue) (Game|Player|GetHitResultUnderCursorbyChannel "TraceTypeQuery1" true))
  (bind _returnvalue_2 (Pawn|GetControlledPawn))
  (bind _dmi_cursor (Variables|Default|GetDMI_Cursor))
  (bind (_x _y) (Math|Vector|BreakVector (.location _hitresult)))
  (bind _returnvalue_3 (Transformation|GetActorLocation _returnvalue_2))
  (:Started
    (bind _pathfindervolume (Class|IGameState|IGetPathFinderVolume(Message) (Game|GetGameState)))
    (if (and _returnvalue (Variables|Default|GetbCursorAttack))
      (Class|BPICharacter|MoveCharacter(Message) (Pawn|GetControlledPawn) (Class|PathFinderVolume|GetGridArrayIndexbyLocation _pathfindervolume (Math|Vector2D|MakeVector2D (.x _returnvalue_3) (.y _returnvalue_3))) (Class|PathFinderVolume|GetGridArrayIndexbyLocation _pathfindervolume (Math|Vector2D|MakeVector2D _x _y)) (Math|Vector2D|MakeVector2D _x _y) true)
      (Variables|Default|SetbCursorAttack false)
      (bind _asgohudbase (Utilities|Casting|CastToGOHUDBase (HUD|GetHUD)))
      (Class|GOHUDBase|OnChangeMouseCursorTypeImplementation _asgohudbase "/Script/ProjectGO.GODefaultCursorType")
      (bind _returnvalue_4 (Niagara|SpawnSystematLocation (Variables|Default|GetFXCursor) (.location _hitresult)))
      (Class|NiagaraComponent|SetVariableMaterial _returnvalue_4 "DynamicMaterial" _dmi_cursor)
      (Rendering|Material|SetVectorParameterValue _dmi_cursor "Color" "(R=255.000000,G=0.000000,B=0.000000,A=1.000000)" :!class /Script/Engine.MaterialInstanceDynamic))))

(event Input|EnhancedActionEvents|EnhancedInputActionIA_AttributeWidgetOpen
  (params (ActionValue :type Boolean) (ElapsedSeconds :type Float%20%28double-precision%29) (TriggeredSeconds :type Float%20%28double-precision%29) (InputAction :type Input%20Action%20Object%20Reference :default "/Game/Input/Actions/IA_AttributeWidgetOpen.IA_AttributeWidgetOpen"))
  (:Started
    (bind _returnvalue (UserInterface|CreateWidget "/Game/UI/AttributeMenu/WBP_AttributeMenu.WBP_AttributeMenu_C" self))
    (Input|SetInputModeUIOnly self _returnvalue "LockAlways" true)
    (UserInterface|Viewport|AddtoViewport _returnvalue 0)))

(event EventBeginPlay
  (|CallParentFunction)
  (bind _returnvalue (Rendering|Material|CreateDynamicMaterialInstance "/Game/Cursor/MI_Cursor_Inst.MI_Cursor_Inst" "None" "None" :!class /Script/Engine.KismetMaterialLibrary))
  (Variables|Default|SetDMI_Cursor _returnvalue))

(event Input|MouseEvents|MouseWheelAxis
  (params (AxisValue :type Float%20%28single-precision%29))
  (bind _asgoplayer_camera_manager (Utilities|Casting|CastToGOPlayerCameraManager (Game|GetPlayerCameraManager 0)))
  (Class|GOPlayerCameraManager|SetCameraFOVSmooth _asgoplayer_camera_manager AxisValue))

(event Input|MouseEvents|MouseX
  (params (AxisValue :type Float%20%28single-precision%29))
  (bind _asgoplayer_camera_manager (Utilities|Casting|CastToGOPlayerCameraManager (Game|GetPlayerCameraManager 0)))
  (Class|GOPlayerCameraManager|CameraMoveMouseX _asgoplayer_camera_manager))

(event Input|MouseEvents|MouseY
  (params (AxisValue :type Float%20%28single-precision%29))
  (bind _asgoplayer_camera_manager (Utilities|Casting|CastToGOPlayerCameraManager (Game|GetPlayerCameraManager 0)))
  (Class|GOPlayerCameraManager|CameraMoveMouseY _asgoplayer_camera_manager))

(fn ConstructionScript
  (|CallParentFunction))