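; BP_PathFindVolume is a placed volume that builds a walkability grid for pathfinding.
; Its construction script computes cell-center points from map size, grid size and actor location; the debug box drawing is disconnected.
; The CreatePathFindGridActors event sphere-traces each point against WorldStatic objects and stores row, column, location and walkability through SetGrids.
; Despite its name, that event spawns no actors, and it prints each cell for debugging.
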(event Custom|CreatePathFindGridActors
  (bind _returnvalue (Transformation|GetActorLocation))
  (bind _gridsize (Variables|Default|GetGridSize))
  (bind _mapsize (Variables|Default|GetMapSize))
  (bind _returnvalue_2 (/ (.x _mapsize) (.x _gridsize)))
  (Utilities|Array|Clear (Class|PathFinderVolume|GetGrids))
  (for (_array_element _array_index) (Variables|Default|GetVector_GridArray)
    (bind _returnvalue_3 (Collision|SphereTraceForObjects (Math|Vector|MakeVector (.x _array_element) (.y _array_element) (+ (.z _returnvalue) 1e+02)) (Math|Vector|MakeVector (.x _array_element) (.y _array_element) (+ (.z _returnvalue) 2e+02)) (.x _gridsize) (Utilities|Array|MakeArray "ObjectTypeQuery1") false 0 "ForDuration"))
    (Utilities|Array|Add (Variables|Default|GetNewGridsArr) (Utilities|Struct|MakePathFindGridInfo (/ _array_index _returnvalue_2) (Math|Integer|%(Integer) _array_index _returnvalue_2) (not _returnvalue_3) (Math|Vector2D|MakeVector2D (.x _array_element) (.y _array_element))))
    (Development|PrintString (Utilities|String|Append (Utilities|String|ToString(Integer) (/ _array_index _returnvalue_2)) "  ///  " (Utilities|String|ToString(Integer) (Math|Integer|%(Integer) _array_index _returnvalue_2)) "   ///   " (Utilities|String|ToString(Vector2d) (Math|Vector2D|MakeVector2D (.x _array_element) (.y _array_element))))))
  (Class|PathFinderVolume|SetGrids (Variables|Default|GetNewGridsArr)))

(event EventBeginPlay
  (|CallParentFunction))

(event Collision|EventActorBeginOverlap
  (params (OtherActor :type Actor%20Object%20Reference)))

(event EventTick
  (params (DeltaSeconds :type Float%20%28single-precision%29)))

(fn ConstructionScript
  (bind _gridsize (Variables|Default|GetGridSize))
  (bind _gridsize_2 (Variables|Default|GetGridSize))
  (bind _mapsize (Variables|Default|GetMapSize))
  (|CallParentFunction)
  (Utilities|Array|Clear (Variables|Default|GetVector_GridArray))
  (Rendering|Debug|FlushPersistentDebugLines)
  (LocalVariables|SetRowCount (/ (.y _mapsize) (.y _gridsize_2)))
  (LocalVariables|SetColCount (/ (.x _mapsize) (.x _gridsize_2)))
  (for _index (range 0 (- (LocalVariables|GetRowCount) 1))
    (for _index_2 (range 0 (- (LocalVariables|GetColCount) 1))
      (Utilities|Array|Add (Variables|Default|GetVector_GridArray) (Math|Vector2D|MakeVector2D (.x (+ (Math|Conversions|ToVector2D(Vector) (Transformation|GetActorLocation)) (Math|Vector2D|MakeVector2D (+ (* _index (.y _gridsize) 2.0) (.y _gridsize)) (+ (* _index_2 (.x _gridsize) 2.0) (.x _gridsize))))) (.y (+ (Math|Conversions|ToVector2D(Vector) (Transformation|GetActorLocation)) (Math|Vector2D|MakeVector2D (+ (* _index (.y _gridsize) 2.0) (.y _gridsize)) (+ (* _index_2 (.x _gridsize) 2.0) (.x _gridsize))))))))))