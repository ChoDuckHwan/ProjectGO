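; BP_PathFindGrid is a pathfinding grid cell that works out at startup whether it can be moved through.
; After the parent BeginPlay, it traces a short line straight up from its location for WorldStatic objects.
; On a hit it prints the blocking actor's name, reports its Row and Col as blocked through SetGridInfo and clears CanMove.
; Otherwise it only sets CanMove to true.
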(event EventBeginPlay
  (bind _returnvalue (Transformation|GetActorLocation))
  (|CallParentFunction)
  (bind (_outhit _returnvalue_2) (Collision|LineTraceForObjects (Transformation|GetActorLocation) (Math|Vector|MakeVector (.x _returnvalue) (.y _returnvalue) (+ (.z _returnvalue) 1e+02)) (Utilities|Array|MakeArray "ObjectTypeQuery1") false 0 "None"))
  (if _returnvalue_2
    (Development|PrintString (Utilities|GetDisplayName (.HitActor (Collision|BreakHitResult _outhit))))
    (Class|PathFindGrid|SetGridInfo (Utilities|Struct|MakePathFinGridInfo (Variables|Default|GetRow) (Variables|Default|GetCol) false))
    (Variables|Default|SetcanMove false)
    (else
      (Variables|Default|SetcanMove true))))

(fn ConstructionScript)